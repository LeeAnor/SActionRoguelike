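; Game mode Blueprint for an action roguelike, holding an unfinished EQS-driven spawner for MinionRush_BP bots.
; Disconnected nodes set a looping timer, run the bot spawn location query in random best 25% mode, and bind its finished event.
; That event spawns a minion at the first returned location if it passes a validity check.
; BeginPlay is empty, with a note that a loop is still needed, so spawning never starts.
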(event Custom|OnQueryFinishedEvent_事件_0
  (params (QueryInstance :type Env%20Query%20Instance%20Blueprint%20Wrapper%20Object%20Reference) (QueryStatus :type EEnvQueryStatus%20Enum :default "Processing"))
  (Development|PrintString "finish eqs query")
  (bind _resultlocations (AI|EQS|GetQueryResultsasLocations QueryInstance))
  (if (AI|IsValidAILocation (Utilities|Array|Get(acopy) _resultlocations))
    (Game|SpawnActorfromClass "/Game/ActionRoguelike/AI/MinionRushed/MinionRush_BP.MinionRush_BP_C" (Math|Transform|MakeTransform (Utilities|Array|Get(acopy) _resultlocations)) "Undefined" 0 0)))

(event EventBeginPlay
  ;[1 1 1] 这里应该创建一个循环，但是我不知道怎么创建
)

(fn ConstructionScript)