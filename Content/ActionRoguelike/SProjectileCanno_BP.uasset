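; A projectile cannon actor that periodically fires magic projectiles.
; On BeginPlay it starts a looping timer that spawns BP_MagicProjectile at the actor's location and rotation.
; Each Tick it turns its Arrow component to face the first player's pawn, when valid.
; The spawn reads the actor's rotation rather than the Arrow's, so shots follow that aim only if Arrow is the root component.
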(event Custom|EmitProjectile
  (Game|SpawnActorfromClass "/Game/ActionRoguelike/Projectile/BP_MagicProjectile.BP_MagicProjectile_C" (Math|Transform|MakeTransform (Transformation|GetActorLocation) (Transformation|GetActorRotation)) "Undefined" 0 0))

(event EventBeginPlay
  (Utilities|Time|SetTimerbyEvent (delegate Custom|EmitProjectile) 2.0 true))

(event EventTick
  (params (DeltaSeconds :type Float%20%28single-precision%29))
  (bind _returnvalue (Game|Player|GetPlayerPawn 0))
  (Utilities|IsValid _returnvalue
    (:Is%20Valid
      (Transformation|SetWorldRotation (Variables|Default|GetArrow) (Math|Rotator|FindLookatRotation (Transformation|GetActorLocation) (Transformation|GetActorLocation _returnvalue)) false false))))

(fn ConstructionScript)